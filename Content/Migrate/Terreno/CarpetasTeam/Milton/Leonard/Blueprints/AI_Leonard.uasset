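; AI controller for the Leonard character that starts its behavior tree when play begins.
; On BeginPlay it loads Leonard's blackboard and fills seven position keys: the first with the controlled pawn's starting location, the rest from position variables on the controller.
; It then runs Leonard_BehaviorTree, which receives those points through the blackboard; the controller has no other active logic.
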(event `self.ReceiveBeginPlay`
  (bind _blackboardcomponent (`self.UseBlackboard` "/Game/Migrate/Terreno/CarpetasTeam/Milton/Leonard/Blueprints/Leonard_Blackboard.Leonard_Blackboard"))
  (`BlackboardComponent.SetValueAsVector` _blackboardcomponent "Posicion1" (`self.K2_GetActorLocation` (`self.K2_GetPawn`)))
  (`BlackboardComponent.SetValueAsVector` _blackboardcomponent "Posicion2" (`self.Posicion2`))
  (`BlackboardComponent.SetValueAsVector` _blackboardcomponent "Posicion3" (`self.Posicion3`))
  (`BlackboardComponent.SetValueAsVector` _blackboardcomponent "Posicion4" (`self.Posicion4`))
  (`BlackboardComponent.SetValueAsVector` _blackboardcomponent "Posicion5" (`self.Posicion5`))
  (`BlackboardComponent.SetValueAsVector` _blackboardcomponent "Posicion6" (`self.Posicion6`))
  (`BlackboardComponent.SetValueAsVector` _blackboardcomponent "Posicion7" (`self.Posicion7`))
  (`self.RunBehaviorTree` "/Game/Migrate/Terreno/CarpetasTeam/Milton/Leonard/Blueprints/Leonard_BehaviorTree.Leonard_BehaviorTree"))

(fn `UserConstructionScript`)